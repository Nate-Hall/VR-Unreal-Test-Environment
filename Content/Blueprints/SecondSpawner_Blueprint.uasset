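; SecondSpawner is a spawner actor that creates a row of BP_PickupCube pickups when play begins.
; A BeginPlay loop steps an offset along world Y, starting behind the actor's location, and spawns evenly spaced cubes owned by the spawner.
; Each integer-truncated world position also passes through TransformLocation with the actor's own transform, so the actor's translation, rotation and scale apply on top of it.
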(event `self.ReceiveBeginPlay`
  (set `self.count` 0)
  (while (< (`self.count`) 400)
    (`|SpawnActorFromClass` "/Game/VirtualRealityBP/Blueprints/BP_PickupCube.BP_PickupCube_C" (`KismetMathLibrary.Conv_VectorToTransform` (`KismetMathLibrary.TransformLocation` (`self.GetTransform`) (`KismetMathLibrary.Conv_IntVectorToVector` (make `IntVector` (`KismetMathLibrary.FTrunc` (.x (`self.K2_GetActorLocation`))) (`KismetMathLibrary.FTrunc` (+ (- (.y (`self.K2_GetActorLocation`)) 200.0) (`KismetMathLibrary.Conv_IntToDouble` (`self.count`)))) (`KismetMathLibrary.FTrunc` (.z (`self.K2_GetActorLocation`))))))) "Undefined" "OverrideRootScale" self null)
    (set `self.count` (`KismetMathLibrary.FTrunc` (+ (`KismetMathLibrary.Conv_IntToDouble` (`self.count`)) 40.0)))))

(fn `UserConstructionScript`)